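; BP_ImageStreaming is an actor that shows an image downloaded from a URL on a plane mesh.
; Its construction script creates a dynamic material instance of MM_ImageStreaming on the plane.
; Subscribe callbacks set the image URL and trigger downloads, which the UpdateImage event can also start.
; Each successful download replaces the material's Texture parameter, with no handling for failures.
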(event Custom|Update%20Image
  (bind _texture (|DownloadImage (Variables|Default|GetImage%20URL))
    (:OnSuccess
      (Rendering|Material|SetTextureParameterValue (Variables|Default|GetPlane%20Material) "Texture" _texture))))

(fn ConstructionScript
  (bind _returnvalue (Rendering|Material|CreateDynamicMaterialInstance (Variables|Default|GetPlane) 0 "/Game/ImageStreamer/MM_ImageStreaming.MM_ImageStreaming" "None" :!class /Script/Engine.PrimitiveComponent))
  (Variables|Default|SetPlane%20Material _returnvalue))